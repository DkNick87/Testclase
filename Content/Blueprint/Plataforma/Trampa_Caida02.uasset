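; Trap platform that sends the player back to their starting location on contact.
; On BeginPlay it stores the player pawn's location and plays a timeline that moves the Cube and Box along Z at a fixed, hard-coded world XY.
; Any overlap with the Box teleports player 0 to that stored location unless the pawn is falling, without checking which actor overlapped.
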(event OnComponentBeginOverlap(Box)
  (params (OverlappedComponent :type Primitive%20Component%20Object%20Reference) (OtherActor :type Actor%20Object%20Reference) (OtherComp :type Primitive%20Component%20Object%20Reference) (OtherBodyIndex :type Integer) (bFromSweep :type Boolean) (SweepResult :type Hit%20Result%20Structure%20%28by%20ref%29))
  ;[1 1 1] Trampa_traslado de pj 2parte. variable Vector arriba, para automatico
  (if (not (AI|Components|NavMovement|IsFalling (Pawn|GetMovementComponent (Game|Player|GetPlayerPawn 0))))
    (Transformation|SetActorLocation (Game|Player|GetPlayerPawn 0) (Variables|Default|GetPosicionInicial) false false)))

(event EventBeginPlay
  ;[1 1 1] Traslacion de la plataforma
  ;;[1 1 1] Traslado pj por box
  (Variables|Default|SetPosicionInicial (Transformation|GetActorLocation (Game|Player|GetPlayerPawn 0)))
  (bind _newtrack_0 (Timeline|Traslado%20Plataforma Play)
    (:Update
      (Transformation|SetWorldLocation (Variables|Default|GetCube) (Math|Vector|MakeVector -8.6e+02 1.22e+03 _newtrack_0) false false))))

(event Collision|EventActorBeginOverlap
  (params (OtherActor :type Actor%20Object%20Reference)))

(event EventTick
  (params (DeltaSeconds :type Float%20%28single-precision%29)))

(fn ConstructionScript)